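; Melee enemy character for a wave mode that chases the player and pushes them for damage, wearing a random mesh.
; AI MoveTo leads into a push montage whose notify sphere-traces for pawns to damage, then chasing resumes on completion.
; Damage knocks it back; at zero health it ragdolls, calls BP_WaveSpawned's enemy check after a delay and destroys itself.
; A looping random Wonder movement event exists but is never called here.
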(event `self.ReceiveBeginPlay`
  (`self.ChasePlayer`)
  (`SkeletalMeshComponent.SetSkeletalMeshAsset` (`self.Mesh`) (`KismetArrayLibrary.Array_Random` (`self.Meshes`))))

(event `ChasePlayer`
  (bind _attackpostion (`self.AttackPostion`))
  (bind _returnvalue (`SceneComponent.K2_GetComponentLocation` _attackpostion))
  ;[0.2917 0.2917 0.2917] Chase Player
  (`|AIMoveTo` self (0.0 0.0 0.0) (`GameplayStatics.GetPlayerCharacter` 0)
    (:`OnSuccess`
      (if (`self.CanAttack`)
        (`|PlayMontage` (`self.Mesh`) "/Game/Characters/Mannequin_UE4/OurAnimations/Push_Montage.Push_Montage"
          (:`then`
            (set `self.CanAttack` false))
          (:`OnCompleted`
            (set `self.CanAttack` true)
            (`self.ChasePlayer`))
          (:`OnNotifyBegin`
            (bind (_outhit _returnvalue_2) (`KismetSystemLibrary.SphereTraceSingleForObjects` _returnvalue (+ _returnvalue (* (`SceneComponent.GetForwardVector` _attackpostion) 100.0)) 25.0 (`|MakeArray` "ObjectTypeQuery3" :!type "EObjectTypeQuery Enum")))
            (if _returnvalue_2
              (`GameplayStatics.ApplyDamage` (`.HitActor` (`GameplayStatics.BreakHitResult` _outhit)) 10.0))))))
    (:`OnFail`
      (`KismetSystemLibrary.PrintString` "enemy going wrong"))))

(event `Wonder`
  ;[0.2917 0.2917 0.2917] Wonder
  (`|AIMoveTo` self (`NavigationSystemV1.K2_GetRandomReachablePointInRadius` (`self.K2_GetActorLocation`) 500.0 null null) null
    (:`then`
      (`KismetSystemLibrary.Delay` 1.0)
      (`self.Wonder`))))

(event `self.ReceiveAnyDamage`
  (params (Damage :type "Float (single-precision)") (DamageType :type "DamageType Object Reference") (InstigatedBy :type "Controller Object Reference") (DamageCauser :type "Actor Object Reference"))
  ;[0.2917 0.2917 0.2917] Damage
  (bind _output_get (set `self.Health` (- (`self.Health`) Damage)))
  (`GameplayStatics.PlaySoundAtLocation` "/Game/Sound/Ms_Damage.Ms_Damage" (`self.K2_GetActorLocation`) (struct) 1.0 1.0 0.0 null null null null)
  (if (<= _output_get 0.0)
    (`PrimitiveComponent.SetSimulatePhysics` (`self.Mesh`) true)
    (set `self.CanAttack` false)
    (`CharacterMovementComponent.DisableMovement` (`self.CharacterMovement`))
    (`KismetSystemLibrary.Delay` 3.0)
    (bind _returnvalue (`GameplayStatics.GetActorOfClass` "/Game/BluePrints/BP_WaveSpawned.BP_WaveSpawned_C"))
    (`/Game/BluePrints/BP_WaveSpawned.Check for enemies` _returnvalue)
    (`self.K2_DestroyActor`)
    (else
      (`self.LaunchCharacter` (+ (* (`self.GetActorForwardVector`) -200.0) (* (`self.GetActorUpVector`) 100.0))))))

(fn `UserConstructionScript`)