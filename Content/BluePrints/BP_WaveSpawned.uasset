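; BP_WaveSpawned is a wave manager that spawns successive waves of BP_Enemy, starting at BeginPlay.
; SpawnWave plays a sound, increments the wave counter and uses the matching entry from the Waves map values as the enemy count, placing each at a random SpawnedWavePositions transform.
; Checkforenemies, not called within this Blueprint, waits briefly, then starts the next wave and prints a debug string if no enemies remain.
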(event `self.ReceiveBeginPlay`
  (`self.Spawn Wave`))

(event `Spawn Wave`
  (`GameplayStatics.PlaySound2D` "/Game/Sound/Wave.Wave" 1.0 1.0 0.0 null null)
  (`/Engine/EditorBlueprintResources/StandardMacros.IncrementInt` (`self.CurrentValue`)
    (:`  `
      (bind _values (`BlueprintMapLibrary.Map_Values` (`self.Waves`)))
      (for _ (range 1 (+ (`|GetArrayItem` _values (- (`self.CurrentValue`) 1)) 1))
        (`|SpawnActorFromClass` "/Game/BluePrints/BP_Enemy.BP_Enemy_C" (`KismetArrayLibrary.Array_Random` (`self.Spawned Wave Positions`)) "AdjustIfPossibleButDontSpawnIfColliding" "MultiplyWithRoot" null null)))))

(event `Check for enemies`
  (`KismetSystemLibrary.Delay` 0.2)
  (bind _outactors (`GameplayStatics.GetAllActorsOfClass` "/Game/BluePrints/BP_Enemy.BP_Enemy_C"))
  (if (== (`KismetArrayLibrary.Array_Length` _outactors) 0)
    (`self.Spawn Wave`)
    (`KismetSystemLibrary.PrintString` "Hello")))

(fn `UserConstructionScript`)